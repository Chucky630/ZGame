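; BP_PowerBase is an enum-driven power system actor acting as a light, switch, power box or power station.
; Construction sets the mesh or light intensity per type, while Interaction branches on the same enum.
; Switches toggle the lights in their PoweredObjects array unless the box is off.
; Boxes propagate PowerBoxOff to their powered objects and call their LightsOn/LightsOff; stations have no interaction logic.
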(fn `Interaction`
  (returns (True :type Boolean))
  (bind _poweredobjects (`self.PoweredObjects`))
  ;[1 1 1] Change Function Depending On Enum
  (switch `/Game/GameContent/PowerSystem/Power_Enum` (`self.PowerEnum`)
    (:`NewEnumerator0`
      ;[1 1 1] Light Function
      (`KismetSystemLibrary.PrintString` "Light"))
    (:`NewEnumerator1`
      (`KismetSystemLibrary.PrintString` "Swtich")
      ;[1 1 1] Light Switch
      (if (not (`self.PowerBoxOff`))
        ;;[1 1 1] Check if the Power is off?
        (if (`self.PowerOff`)
          (`self.Lights On`)
          (set `self.PowerOff` false)
          (else
            (`self.Lights off`)
            (set `self.PowerOff` true)))))
    (:`NewEnumerator2`
      (`KismetSystemLibrary.PrintString` "Box")
      ;[1 1 1] PowerBox
      (if (`self.PowerBoxOff`)
        (set `self.PowerBoxOff` false)
        (for _array_element _poweredobjects
          (set `/Game/GameContent/PowerSystem/BP_PowerBase.PowerBoxOff` false _array_element)
          (`self.Lights On` _array_element))
        (else
          (set `self.PowerBoxOff` true)
          (for _array_element_2 _poweredobjects
            (set `/Game/GameContent/PowerSystem/BP_PowerBase.PowerBoxOff` true _array_element_2)
            (`self.Lights off` _array_element_2)))))))

(fn `Lights off`
  ;[1 1 1] Depending on If the power is off or not, Gets all Actors in the array, and sets the Light intensity to 0 or 5000
  (for _array_element (`self.PoweredObjects`)
    (`LightComponent.SetIntensity` (`/Game/GameContent/PowerSystem/BP_PowerBase.PointLight` _array_element) 0.0)))

(fn `Lights On`
  (`KismetSystemLibrary.PrintString` "on")
  (for _array_element (`self.PoweredObjects`)
    (`LightComponent.SetIntensity` (`/Game/GameContent/PowerSystem/BP_PowerBase.PointLight` _array_element) 100.0)))

(fn `UserConstructionScript`
  (bind _staticmesh (`self.StaticMesh`))
  (`/Engine/EditorBlueprintResources/StandardMacros.DoOnce` false
    (:`Completed`
      (switch `/Game/GameContent/PowerSystem/Power_Enum` (`self.PowerEnum`)
        (:`NewEnumerator0`
          (`LightComponent.SetIntensity` (`self.PointLight`) 100.0)
          (`StaticMeshComponent.SetStaticMesh` _staticmesh null))
        (:`NewEnumerator1`
          (`StaticMeshComponent.SetStaticMesh` _staticmesh "/Game/Models/PowerSystem/LightSwitch.LightSwitch"))
        (:`NewEnumerator2`
          (`StaticMeshComponent.SetStaticMesh` _staticmesh "/Game/Models/PowerSystem/PowerBox_House_.PowerBox_House_"))
        (:`NewEnumerator3`
          (`StaticMeshComponent.SetStaticMesh` _staticmesh "/Game/Models/PowerSystem/PowerBox_Street_.PowerBox_Street_"))))))