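; Placeable spawn point that creates a car, loot chest, zombie or survivor, chosen by SpawnEnum.
; Car points show a placeholder vehicle mesh from the Construction Script, then on BeginPlay clear it and spawn a random class from VehicleDataTable at the root's relative location.
; The other types spawn their configured class directly from the Construction Script at the root's world transform, with no BeginPlay step.
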(event `self.ReceiveBeginPlay`
  (switch `/Game/GameContent/Spawning/SpawnerType_Enum` (`self.SpawnEnum`)
    (:`NewEnumerator0`
      (`self.VehicleSpawn`))))

(fn `LootChestSpawn`
  (`|SpawnActorFromClass` (`self.LootChestClass`) (`SceneComponent.K2_GetComponentToWorld` (`self.DefaultSceneRoot`)) "Undefined" "OverrideRootScale" null null))

(fn `SurvivorSpawn`
  (`|SpawnActorFromClass` (`self.SurvivorClass`) (`SceneComponent.K2_GetComponentToWorld` (`self.DefaultSceneRoot`)) "Undefined" "OverrideRootScale" null null))

(fn `UserConstructionScript`
  (switch `/Game/GameContent/Spawning/SpawnerType_Enum` (`self.SpawnEnum`)
    (:`NewEnumerator0`
      (`SkeletalMeshComponent.SetSkeletalMeshAsset` (`self.SkeletalMesh`) "/Game/Models/Vehicle/SM_SimpleVehicle.SM_SimpleVehicle"))
    (:`NewEnumerator1`
      (`self.LootChestSpawn`))
    (:`NewEnumerator2`
      (`self.ZombieSpawn`))
    (:`NewEnumerator3`
      (`self.SurvivorSpawn`))))

(fn `VehicleSpawn`
  (`SkeletalMeshComponent.SetSkeletalMeshAsset` (`self.SkeletalMesh`) null)
  (bind _outrownames (`DataTableFunctionLibrary.GetDataTableRowNames` "/Game/GameContent/Spawning/VehicleDataTable.VehicleDataTable"))
  (bind _returnvalue (`|GetDataTableRow` "/Game/GameContent/Spawning/VehicleDataTable.VehicleDataTable" (`KismetArrayLibrary.Array_Random` _outrownames))
    (:`then`
      (`|SpawnActorFromClass` (`.VehicleClass_19_15E8BEF64826DC3B5C2FC4B4568A0BE8` (break `/Game/GameContent/Spawning/Vehicle_Struct` _returnvalue)) (`KismetMathLibrary.MakeTransform` (`SceneComponent.RelativeLocation` (`self.DefaultSceneRoot`))) "Undefined" "OverrideRootScale" null null))))

(fn `ZombieSpawn`
  (`|SpawnActorFromClass` (`self.ZombieClass`) (`SceneComponent.K2_GetComponentToWorld` (`self.DefaultSceneRoot`)) "Undefined" "OverrideRootScale" null null))