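; BP_ItemBase is a world item, apparently a base for pickups, that the player adds to their inventory through Interaction.
; Its construction script looks up RowName in ItemDataTable to set the static mesh and Weight.
; Interaction casts player 0 to BP_ThirdPersonCharacter, passes RowName and Amount to the inventory component, and adds Weight to PlayerWeight.
; Weight is not scaled by Amount, and the actor is not destroyed here.
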(fn `Interaction`
  (returns (True :type Boolean))
  (bind _asbp_third_person_character (cast `/Game/ThirdPerson/Blueprints/BP_ThirdPersonCharacter` (`GameplayStatics.GetPlayerCharacter` 0)))
  (bind _bpc_inventory (`/Game/ThirdPerson/Blueprints/BP_ThirdPersonCharacter.BPC_Inventory` _asbp_third_person_character))
  (`/Game/GameContent/Inventory/BPC_Inventory.AddToInventory` _bpc_inventory (`self.Row Name`) (`self.Amount`))
  (set `/Game/GameContent/Inventory/BPC_Inventory.PlayerWeight` (+ (`/Game/GameContent/Inventory/BPC_Inventory.PlayerWeight` _bpc_inventory) (`self.Weight`)) _bpc_inventory))

(fn `UserConstructionScript`
  (bind _returnvalue (`|GetDataTableRow` "/Game/GameContent/Inventory/ItemDataTable.ItemDataTable" (`self.Row Name`))
    (:`then`
      (bind (_displayname _description _thumbnail _3dmesh _weight) (break `/Game/GameContent/Inventory/ItemStruct` _returnvalue))
      (`StaticMeshComponent.SetStaticMesh` (`self.StaticMesh`) _3dmesh)
      (set `self.Weight` _weight))))